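; BP_RepulsiveArea is an area actor that sends an explosion hit to nearby characters when any actor overlaps it.
; On the server, the overlap draws a debug sphere and runs a sphere query for BP_BaseCharacter pawns within ExplosionRadius.
; Each result implementing BPI_HitInterface receives ExplosionHitMessage with the area's location, strength multiplier and instigator, leaving the reaction to the receiver.
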(event `self.ReceiveActorBeginOverlap`
  (params (OtherActor :type "Actor Object Reference"))
  (`/Engine/EditorBlueprintResources/ActorMacros.Switch Has Authority`
    (:`Authority`
      (`KismetSystemLibrary.DrawDebugSphere` (`self.K2_GetActorLocation`) (`self.ExplosionRadius`) 12 (struct :`G` 1.0 :`B` 0.054741 :`A` 1.0) 3.0 1.0)
      (bind _outactors (`KismetSystemLibrary.SphereOverlapActors` (`self.K2_GetActorLocation`) (`self.ExplosionRadius`) (`|MakeArray` "ObjectTypeQuery3" :!type "EObjectTypeQuery Enum") "/Game/MyContent/Blueprints/Character/BP_BaseCharacter.BP_BaseCharacter_C"))
      (for _array_element _outactors
        (if (`KismetSystemLibrary.DoesImplementInterface` _array_element "/Game/MyContent/Blueprints/BPI_HitInterface.BPI_HitInterface_C")
          (message `/Game/MyContent/Blueprints/BPI_HitInterface.ExplosionHit` _array_element (`self.K2_GetActorLocation`) (`self.StrengthExplosionMultiplier`) (`self.GetInstigator`)))))))

(fn `UserConstructionScript`
  (`parent.UserConstructionScript`))