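; BP_FireArea is an area hazard whose box volume applies and clears damage effects on actors that implement BPI_HitInterface.
; On overlap begin, the server sends a hit message carrying the ArrowType damage type and the area's instigator.
; On overlap end, the server reads the Types array from ArrowType's class defaults and sends a stop-tick-damage message for each entry.
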(event `self.ReceiveBeginPlay`)

(event `self.Box.OnComponentBeginOverlap`
  (params (OverlappedComponent :type "PrimitiveComponent Object Reference") (OtherActor :type "Actor Object Reference") (OtherComp :type "PrimitiveComponent Object Reference") (OtherBodyIndex :type Integer) (bFromSweep :type Boolean) (SweepResult :type "HitResult Structure (by ref)"))
  (`/Engine/EditorBlueprintResources/ActorMacros.Switch Has Authority`
    (:`Authority`
      (if (`KismetSystemLibrary.DoesImplementInterface` OtherActor "/Game/MyContent/Blueprints/BPI_HitInterface.BPI_HitInterface_C")
        (message `/Game/MyContent/Blueprints/BPI_HitInterface.GetHit` OtherActor (`self.ArrowType`) (`self.GetInstigator`))))))

(event `self.Box.OnComponentEndOverlap`
  (params (OverlappedComponent :type "PrimitiveComponent Object Reference") (OtherActor :type "Actor Object Reference") (OtherComp :type "PrimitiveComponent Object Reference") (OtherBodyIndex :type Integer))
  (`/Engine/EditorBlueprintResources/ActorMacros.Switch Has Authority`
    (:`Authority`
      (if (`KismetSystemLibrary.DoesImplementInterface` OtherActor "/Game/MyContent/Blueprints/BPI_HitInterface.BPI_HitInterface_C")
        (for _array_element (defaults `Object` (`self.ArrowType`))
          (message `/Game/MyContent/Blueprints/BPI_HitInterface.StopTickDamage` OtherActor _array_element))))))

(fn `UserConstructionScript`
  (`parent.UserConstructionScript`))