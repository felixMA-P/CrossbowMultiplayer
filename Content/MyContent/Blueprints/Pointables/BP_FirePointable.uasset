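; BP_FirePointable is a pointable target actor that awards points and reacts to hits from a matching arrow type.
; GetHit passes the damage type to AddPoints on the instigating character, whether or not it matches.
; On the authority, a hit matching its TypeArrow triggers the Niagara effect event and starts a timer that destroys the actor after TimeToDisappear.
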(event `self.ReceiveActorBeginOverlap`
  (params (OtherActor :type "Actor Object Reference"))
  (`parent.ReceiveActorBeginOverlap` OtherActor))

(event `/Game/MyContent/Blueprints/BPI_HitInterface.GetHit`
  (params (DamageType :type "/Game/MyContent/Blueprints/ArrowTypes/BP_BaseArrow Class Reference") (CharacterInstigator :type "Pawn Object Reference"))
  ;[1 1 1] Effects
  (`self.AddPoints` DamageType CharacterInstigator)
  (`/Engine/EditorBlueprintResources/ActorMacros.Switch Has Authority`
    (:`Authority`
      (if (== DamageType (`self.TypeArrow`))
        (`self.ActivateNiagaraEffect`)
        (`KismetSystemLibrary.K2_SetTimerDelegate` (delegate `CustomEvent`) (`self.TimeToDisappear`))))))

(event `ActivateNiagaraEffect`
  ;[1 1 1] Effects
  (`ActorComponent.Activate` (`self.Niagara`) true))

(event `CustomEvent`
  ;[1 1 1] Effects
  (`self.K2_DestroyActor`))

(fn `UserConstructionScript`
  (`parent.UserConstructionScript`))