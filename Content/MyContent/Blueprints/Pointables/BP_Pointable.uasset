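; Base pointable actor that a character hits with a typed arrow to score points.
; GetHit passes the damage type and instigator to AddPoints, then starts a timer that destroys the actor after a delay, whatever the arrow type.
; Only on authority and with a matching arrow type, AddPoints awards Points through the instigator's PC_Game controller and notifies its Spawner that the pointable was destroyed.
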(event `/Game/MyContent/Blueprints/BPI_HitInterface.GetHit`
  (params (DamageType :type "/Game/MyContent/Blueprints/ArrowTypes/BP_BaseArrow Class Reference") (CharacterInstigator :type "Pawn Object Reference"))
  (`self.AddPoints` DamageType CharacterInstigator)
  (`KismetSystemLibrary.K2_SetTimerDelegate` (delegate `TimeToDestroy`) (`self.TimeToDisappear`)))

(event `TimeToDestroy`
  (`self.K2_DestroyActor`))

(event `AddPoints`
  (params (TypeArrowIn :type "Object Class Reference") (Target :type "Pawn Object Reference"))
  (`/Engine/EditorBlueprintResources/ActorMacros.Switch Has Authority`
    (:`Authority`
      (if (== TypeArrowIn (`self.TypeArrow`))
        (bind _aspc_game (cast `/Game/MyContent/Blueprints/Game/PC_Game` (`Pawn.GetController` Target)))
        (`/Game/MyContent/Blueprints/Game/PC_Game.OnCharacterPoint` _aspc_game (`self.Points`))
        (`/Game/MyContent/Blueprints/Pointables/BP_Spawner.PointableDestroyed` (`self.Spawner`))))))

(fn `UserConstructionScript`)