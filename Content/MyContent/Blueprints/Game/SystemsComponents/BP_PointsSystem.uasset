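; BP_PointsSystem is a game scoring system that tracks kills, deaths and points for each player.
; A map keyed by PlayerController holds an SPoints struct, zeroed for players on Initialize or game entry and removed on exit.
; Kill, death and AddPoints events rebuild and re-add that entry, applying configurable per-kill rewards and per-death penalties.
; GetPointsInArrays returns the map as key and value arrays.
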(event `GetKill`
  (params (PlayerController :type "/Game/MyContent/Blueprints/Game/PC_Game Object Reference"))
  (bind (_kills _deaths _points) (break `/Game/MyContent/Blueprints/Game/SystemsComponents/S_Points` (`BlueprintMapLibrary.Map_Find` (`self.Points`) PlayerController)))
  (`BlueprintMapLibrary.Map_Add` (`self.Points`) PlayerController (make `/Game/MyContent/Blueprints/Game/SystemsComponents/S_Points` (+ _kills 1) _deaths (+ _points (`self.PointsPerKill`)))))

(event `Die`
  (params (PlayerController :type "/Game/MyContent/Blueprints/Game/PC_Game Object Reference"))
  (bind (_kills _deaths _points) (break `/Game/MyContent/Blueprints/Game/SystemsComponents/S_Points` (`BlueprintMapLibrary.Map_Find` (`self.Points`) PlayerController)))
  (`BlueprintMapLibrary.Map_Add` (`self.Points`) PlayerController (make `/Game/MyContent/Blueprints/Game/SystemsComponents/S_Points` _kills (+ _deaths 1) (- _points (`self.PointsPerDeath`)))))

(event `AddPoints`
  (params (PlayerController :type "/Game/MyContent/Blueprints/Game/PC_Game Object Reference (by ref)") (Points :type Integer))
  (bind (_kills _deaths _points) (break `/Game/MyContent/Blueprints/Game/SystemsComponents/S_Points` (`BlueprintMapLibrary.Map_Find` (`self.Points`) PlayerController)))
  (`BlueprintMapLibrary.Map_Add` (`self.Points`) PlayerController (make `/Game/MyContent/Blueprints/Game/SystemsComponents/S_Points` _kills _deaths (+ _points Points))))

(event `Initialize`
  (params (Players :type "Array of /Game/MyContent/Blueprints/Game/PC_Game Object Reference"))
  (for _array_element Players
    (`BlueprintMapLibrary.Map_Add` (`self.Points`) _array_element (make `/Game/MyContent/Blueprints/Game/SystemsComponents/S_Points` 0))))

(event `OnPlayerExitGame`
  (params (PlayerController :type "/Game/MyContent/Blueprints/Game/PC_Game Object Reference (by ref)"))
  (`BlueprintMapLibrary.Map_Remove` (`self.Points`) PlayerController))

(event `OnPlayerEnterGame`
  (params (PlayerController :type "/Game/MyContent/Blueprints/Game/PC_Game Object Reference (by ref)"))
  (`BlueprintMapLibrary.Map_Add` (`self.Points`) PlayerController (make `/Game/MyContent/Blueprints/Game/SystemsComponents/S_Points` 0)))

(fn `GetPointsInArrays`
  (returns (Keys :type "Array of /Game/MyContent/Blueprints/Game/PC_Game Object Reference") (Values :type "Array of /Game/MyContent/Blueprints/Game/SystemsComponents/S_Points Structure"))
  (bind _points (`self.Points`))
  (bind _keys (`BlueprintMapLibrary.Map_Keys` _points))
  (bind _values (`BlueprintMapLibrary.Map_Values` _points))
  (return _keys _values))