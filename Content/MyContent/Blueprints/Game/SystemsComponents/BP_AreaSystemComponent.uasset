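; BP_AreaSystemComponent is a system component that spawns area actors on request and tracks those currently alive.
; AreaTrySpawn looks up a class by key in the AreaClass map and passes it to SpawnArea with location, rotation and instigator.
; SpawnArea always spawns regardless of collision, adds the actor to CurrentAreas and binds its OnDestroyed event, which removes destroyed BP_Area actors from that list.
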(event `SpawnArea`
  (params (Instigator :type "Pawn Object Reference") (Location :type "Vector Structure") (Class :type "/Game/MyContent/Blueprints/Areas/BP_Area Class Reference") (`Spawn Transform Rotation` :type "Rotator Structure"))
  (bind _returnvalue (`|SpawnActorFromClass` Class (`KismetMathLibrary.MakeTransform` Location `Spawn Transform Rotation`) "AlwaysSpawn" "MultiplyWithRoot" null 2.0 Instigator))
  (`/Engine/EditorBlueprintResources/StandardMacros.IsValid` _returnvalue
    (:`Is Valid`
      (add `Actor.OnDestroyed` _returnvalue (delegate `OnDestroyed_Event`))
      (`KismetArrayLibrary.Array_Add` (`self.CurrentAreas`) _returnvalue))))

(event `OnDestroyed_Event`
  (params (DestroyedActor :type "Actor Object Reference"))
  (bind _asbp_area (cast `/Game/MyContent/Blueprints/Areas/BP_Area` DestroyedActor))
  (`KismetArrayLibrary.Array_RemoveItem` (`self.CurrentAreas`) _asbp_area))

(event `AreaTrySpawn`
  (params (Location :type "Vector Structure") (Instigator :type "Pawn Object Reference") (Key :type "/Game/MyContent/Blueprints/E_DamageType Enum (by ref)") (`Spawn Transform Rotation` :type "Rotator Structure"))
  (bind (_value _returnvalue) (`BlueprintMapLibrary.Map_Find` (`self.AreaClass`) Key))
  (if _returnvalue
    (`self.SpawnArea` Instigator Location _value `Spawn Transform Rotation`)))