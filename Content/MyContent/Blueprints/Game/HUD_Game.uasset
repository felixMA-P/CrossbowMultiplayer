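; Game HUD that owns the player's on-screen widgets for health, ammo, arrow quiver, scoreboard, waiting for players and respawn.
; Refresh events forward values to sub-widgets of the main UI through GetMainUI, which lazily creates and caches that widget.
; The waiting-for-players screen is created on first check, updated afterwards and cleared on removal.
; The respawn window is created separately on demand.
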(event `self.ReceiveBeginPlay`
  (`self.GetMainUI`))

(event `RefreshHPBar`
  (params (CurrentHP :type "Float (double-precision)") (MaxHP :type "Float (double-precision)"))
  (bind _w_mainui (`self.GetMainUI`))
  (`/Game/MyContent/UsetInterface/Game/UW_HealthBar.SetPercent` (`/Game/MyContent/UsetInterface/Game/UW_MainUI.UW_HealthBar` _w_mainui) CurrentHP MaxHP))

(event `RefreshMagazineAmmo`
  (params (Ammo :type Integer))
  (bind _w_mainui (`self.GetMainUI`))
  (`/Game/MyContent/UsetInterface/Game/UW_AmmoSystem.UpdateCurrentMagazine` (`/Game/MyContent/UsetInterface/Game/UW_MainUI.UW_AmmoSystem` _w_mainui) Ammo))

(event `RefreshTotalAmmo`
  (params (Ammo :type Integer))
  (bind _w_mainui (`self.GetMainUI`))
  (`/Game/MyContent/UsetInterface/Game/UW_AmmoSystem.UpdateTotalAmmoLeft` (`/Game/MyContent/UsetInterface/Game/UW_MainUI.UW_AmmoSystem` _w_mainui) Ammo))

(event `RefreshSelectedArrow`
  (params (NewSelectedArrow :type "/Game/MyContent/Blueprints/ArrowTypes/BP_BaseArrow Class Reference"))
  (bind _w_mainui (`self.GetMainUI`))
  (`/Game/MyContent/UsetInterface/Game/ArrowSelector/UW_Selector.RefreshSelectedArrow` (`/Game/MyContent/UsetInterface/Game/UW_MainUI.UW_Selector` _w_mainui) NewSelectedArrow))

(event `InitilizeQuiverUI`
  (params (ArrowsQuiverClasses :type "Array of /Game/MyContent/Blueprints/ArrowTypes/BP_BaseArrow Class Reference") (ArrowsQuiverQuant :type "Array of Integer"))
  (bind _w_mainui (`self.GetMainUI`))
  (`/Game/MyContent/UsetInterface/Game/ArrowSelector/UW_Selector.Inicialize` (`/Game/MyContent/UsetInterface/Game/UW_MainUI.UW_Selector` _w_mainui) ArrowsQuiverClasses ArrowsQuiverQuant))

(event `UpdateNumberOfArrowsQuiver`
  (params (TypesOfArrow :type "Array of /Game/MyContent/Blueprints/ArrowTypes/BP_BaseArrow Class Reference") (NumbersOfArrows :type "Array of Integer"))
  (bind _w_mainui (`self.GetMainUI`))
  (`/Game/MyContent/UsetInterface/Game/ArrowSelector/UW_Selector.UpdateNumberOfArrows` (`/Game/MyContent/UsetInterface/Game/UW_MainUI.UW_Selector` _w_mainui) TypesOfArrow NumbersOfArrows))

(event `OpenUIPuntuationTab`
  (params (PlayerControllers :type "Array of String (by ref)") (Points :type "Array of /Game/MyContent/Blueprints/Game/SystemsComponents/S_Points Structure (by ref)"))
  (bind _w_mainui (`self.GetMainUI`))
  (bind _uw_pointstable (`/Game/MyContent/UsetInterface/Game/UW_MainUI.UW_PointsTable` _w_mainui))
  (`/Game/MyContent/UsetInterface/Game/Points/UW_PointsTable.Create Data` _uw_pointstable PlayerControllers Points)
  (`Widget.SetVisibility` _uw_pointstable "Visible"))

(event `ClosePuntuationTab`
  (bind _w_mainui (`self.GetMainUI`))
  (`Widget.SetVisibility` (`/Game/MyContent/UsetInterface/Game/UW_MainUI.UW_PointsTable` _w_mainui) "Hidden"))

(fn `CheckRefreshPlayersReady`
  (params (CurrentPlayers :type Integer) (MaxPlayers :type Integer))
  (`self.W_WaitingForPlayers`
    (:`then`
      (`self.RefreshPlayersReady` CurrentPlayers))
    (:`else`
      (`self.ToggleWaitingForPlayers` MaxPlayers CurrentPlayers))))

(fn `CreateRespawnWindow`
  (bind _returnvalue (`|CreateWidget` "/Game/MyContent/UsetInterface/Game/UW_Respawn.UW_Respawn_C"))
  (bind _output_get (set `self.W_Respawning` _returnvalue))
  (`UserWidget.AddToViewport` _output_get 0))

(fn `GetMainUI`
  (returns (w_MainUI :type "/Game/MyContent/UsetInterface/Game/UW_MainUI Object Reference"))
  (`self.w_MainUI`
    (:`then`
      _)
    (:`else`
      (bind _returnvalue (`|CreateWidget` "/Game/MyContent/UsetInterface/Game/UW_MainUI.UW_MainUI_C"))
      (bind _output_get (set `self.w_MainUI` _returnvalue))
      (`UserWidget.AddToViewport` _output_get 0)))
  (return (`self.w_MainUI`)))

(fn `GetPlayerControllerRef`
  (returns (PC :type "/Game/MyContent/Blueprints/Game/PC_Game Object Reference"))
  (`self.PlayerController`
    (:`then`
      _)
    (:`else`
      (bind _aspc_game (cast `/Game/MyContent/Blueprints/Game/PC_Game` (`GameplayStatics.GetPlayerController` 0)))
      (set `self.PlayerController` _aspc_game)))
  (return (`self.PlayerController`)))

(fn `RefreshPlayersReady`
  (params (CurrentNumberPlayers :type Integer))
  (`/Game/MyContent/UsetInterface/Game/UW_WaitingForPlayers.RefreshNumberOfPlayers` (`self.W_WaitingForPlayers`) CurrentNumberPlayers))

(fn `RemoveWaitingForPlayers`
  (bind _w_waitingforplayers (`self.W_WaitingForPlayers`)
    (:`then`
      (`Widget.RemoveFromParent` _w_waitingforplayers)
      (set `self.W_WaitingForPlayers` null))
    (:`else`)))

(fn `ToggleWaitingForPlayers`
  (params (MaxPlayers :type Integer) (CurrentPlayers :type Integer))
  (bind _returnvalue (`|CreateWidget` "/Game/MyContent/UsetInterface/Game/UW_WaitingForPlayers.UW_WaitingForPlayers_C" null MaxPlayers CurrentPlayers))
  (bind _output_get (set `self.W_WaitingForPlayers` _returnvalue))
  (`UserWidget.AddToViewport` _output_get 0)
  (return))

(fn `UserConstructionScript`)