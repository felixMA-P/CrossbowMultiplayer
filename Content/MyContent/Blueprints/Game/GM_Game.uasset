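; Game mode that holds joining players as spectators until the lobby fills, then tells GS_Game to start the match.
; Waiting players possess a BP_SpectatorCharacter, refresh the waiting count and register with PointsSystem; players arriving after the start get a BP_BaseCharacter.
; It forwards area generation requests to AreasSystem and exposes scores from PointsSystem.
; The GS_Game reference is cast once and cached.
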(event `self.HandleStartingNewPlayer`
  (params (NewPlayer :type "PlayerController Object Reference"))
  (if (`self.bGameStarted`)
    (`self.SpawnCharacter` NewPlayer)
    (else
      (bind _returnvalue (`|SpawnActorFromClass` "/Game/MyContent/Blueprints/Character/BP_SpectatorCharacter.BP_SpectatorCharacter_C" (`KismetMathLibrary.MakeTransform` (300.0 200.0 300.0)) "Undefined" "MultiplyWithRoot" NewPlayer null))
      (`Controller.Possess` NewPlayer _returnvalue)
      (`|ExecutionSequence`
        (:`then_0`
          ;[1 1 1] Spectator UI Refresh
          (`/Game/MyContent/Blueprints/Game/GS_Game.RefreshWaitingForPlayers` (`self.GetGameStateRef`)))
        (:`then_1`
          (bind _returnvalue_2 (`self.GetNumPlayers`))
          (if (== _returnvalue_2 (`self.MaxPlayers`))
            (set `self.bGameStarted` true)
            (`/Game/MyContent/Blueprints/Game/GS_Game.StartGame` (`self.GetGameStateRef`))))
        (:`then_2`
          (bind _aspc_game (cast `/Game/MyContent/Blueprints/Game/PC_Game` NewPlayer))
          (`/Game/MyContent/Blueprints/Game/SystemsComponents/BP_PointsSystem.OnPlayerEnterGame` (`self.PointsSystem`) _aspc_game))))))

(event `AskForGenerateArea`
  (params (Instigator :type "Pawn Object Reference") (Location :type "Vector Structure") (Key :type "/Game/MyContent/Blueprints/E_DamageType Enum (by ref)") (`Spawn Transform Rotation` :type "Rotator Structure"))
  (`/Game/MyContent/Blueprints/Game/SystemsComponents/BP_AreaSystemComponent.AreaTrySpawn` (`self.AreasSystem`) Location Instigator Key `Spawn Transform Rotation`))

(fn `GetGameStateRef`
  (returns (GameState :type "/Game/MyContent/Blueprints/Game/GS_Game Object Reference"))
  (`self.BPGameState`
    (:`then`
      _)
    (:`else`
      (bind _asgs_game (cast `/Game/MyContent/Blueprints/Game/GS_Game` (`GameplayStatics.GetGameState`)))
      (set `self.BPGameState` _asgs_game)))
  (return (`self.BPGameState`)))

(fn `GetPuntuation`
  (returns (Keys :type "Array of /Game/MyContent/Blueprints/Game/PC_Game Object Reference") (Values :type "Array of /Game/MyContent/Blueprints/Game/SystemsComponents/S_Points Structure"))
  (bind (_keys _values) (`/Game/MyContent/Blueprints/Game/SystemsComponents/BP_PointsSystem.GetPointsInArrays` (`self.PointsSystem`)))
  (return _keys _values))

(fn `SpawnCharacter`
  (params (PlayerController :type "PlayerController Object Reference") (PlayerStart :type "Actor Object Reference"))
  (bind _returnvalue (`|SpawnActorFromClass` "/Game/MyContent/Blueprints/Character/BP_BaseCharacter.BP_BaseCharacter_C" (`KismetMathLibrary.MakeTransform` (`self.K2_GetActorLocation` PlayerStart)) "Undefined" "MultiplyWithRoot" PlayerController null))
  (`Controller.Possess` PlayerController _returnvalue))

(fn `UserConstructionScript`)