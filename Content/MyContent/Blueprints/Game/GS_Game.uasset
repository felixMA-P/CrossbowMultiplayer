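; GS_Game is the game state that moves players from waiting into a match and updates their waiting-for-players UI.
; StartGame loops PlayerArray, destroys each controlled pawn, has GM_Game spawn a character for the controller, then notifies its PC_Game.
; RefreshWaitingForPlayers pushes the current player count and the game mode's maximum to every PC_Game.
; GetGameModeRef lazily casts and caches the GM_Game reference.
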(event `StartGame`
  (for _array_element (`self.PlayerArray`)
    (bind _returnvalue (`PlayerState.GetPlayerController` _array_element))
    (`self.K2_DestroyActor` (`Controller.K2_GetPawn` _returnvalue))
    (`/Game/MyContent/Blueprints/Game/GM_Game.SpawnCharacter` (`self.GetGameModeRef`) _returnvalue)
    (bind _aspc_game (cast `/Game/MyContent/Blueprints/Game/PC_Game` _returnvalue))
    (`/Game/MyContent/Blueprints/Game/PC_Game.GameStarted` _aspc_game)))

(event `RefreshWaitingForPlayers`
  (bind _playerarray (`self.PlayerArray`))
  ;[1 1 1] Spectator UI refresh
  (for _array_element _playerarray
    (bind _aspc_game (cast `/Game/MyContent/Blueprints/Game/PC_Game` (`PlayerState.GetPlayerController` _array_element)))
    (`/Game/MyContent/Blueprints/Game/PC_Game.RefreshWaitingForPlayers` _aspc_game (`KismetArrayLibrary.Array_Length` _playerarray) (`/Game/MyContent/Blueprints/Game/GM_Game.MaxPlayers` (`self.GetGameModeRef`)))))

(fn `GetGameModeRef`
  (returns (GameMode :type "/Game/MyContent/Blueprints/Game/GM_Game Object Reference"))
  (`self.GameMode`
    (:`then`
      _)
    (:`else`
      (bind _asgm_game (cast `/Game/MyContent/Blueprints/Game/GM_Game` (`GameplayStatics.GetGameMode`)))
      (set `self.GameMode` _asgm_game)))
  (return (`self.GameMode`)))

(fn `UserConstructionScript`)