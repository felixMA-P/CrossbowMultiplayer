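; Actor component that serves as a character's quiver, tracking how many arrows of each type are available.
; Counts live in the NewAmmo map keyed by arrow type, with functions to query a count or check that at least one remains.
; RechargeArrow takes one arrow out and reports success, while SaveArrow returns one and AddArrows adds a given number.
; It runs no event or tick logic.
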(fn `AddArrows`
  (params (ArrowType :type "/Game/MyContent/Blueprints/DamageTypes/BP_BaseDamage Class Reference") (Number :type Integer))
  (`BlueprintMapLibrary.Map_Add` (`self.NewAmmo`) ArrowType (+ Number (`BlueprintMapLibrary.Map_Find` (`self.NewAmmo`) ArrowType))))

(fn `EnoughAmmoOfType`
  (params (Type :type "/Game/MyContent/Blueprints/DamageTypes/BP_BaseDamage Class Reference"))
  (returns (IsEnough :type Boolean))
  (return (>= (`self.GetCurrentAmmoOfType` Type) 1)))

(fn `GetCurrentAmmoOfType`
  (params (Type :type "/Game/MyContent/Blueprints/DamageTypes/BP_BaseDamage Class Reference"))
  (returns (NumberOfArrows :type Integer))
  (return (`BlueprintMapLibrary.Map_Find` (`self.NewAmmo`) Type)))

(fn `RechargeArrow`
  (params (TypeOfArrow :type "/Game/MyContent/Blueprints/DamageTypes/BP_BaseDamage Class Reference"))
  (returns (Succes :type Boolean))
  (bind _value (`BlueprintMapLibrary.Map_Find` (`self.NewAmmo`) TypeOfArrow))
  (if (>= _value 1)
    (`BlueprintMapLibrary.Map_Add` (`self.NewAmmo`) TypeOfArrow (- _value 1))
    (return true)
    (else
      (return false))))

(fn `SaveArrow`
  (params (Type :type "/Game/MyContent/Blueprints/DamageTypes/BP_BaseDamage Class Reference"))
  (`BlueprintMapLibrary.Map_Add` (`self.NewAmmo`) Type (+ (`BlueprintMapLibrary.Map_Find` (`self.NewAmmo`) Type) 1)))