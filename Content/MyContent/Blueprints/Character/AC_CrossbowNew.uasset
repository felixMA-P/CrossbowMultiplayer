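; Crossbow component for the player character that attaches to the first-person mesh, adds weapon input mappings and sets the rifle anim flag.
; ShootOrder aims from the camera, then a server event sphere-traces the shot and consumes ammo through the owner.
; A multicast spawns the arrow type's visual projectile while the trace result waits out a travel delay.
; Interface targets then receive the arrow type; other hits spawn a static collectable arrow.
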(event `self.ReceiveBeginPlay`
  (bind _returnvalue (pcsubsystem `EnhancedInputLocalPlayerSubsystem` (`/Game/MyContent/Blueprints/Character/BP_BaseCharacter.GetPlayerControllerRef` (`self.GetOwnerBaseCharacterRef`))))
  (`|ExecutionSequence`
    (:`then_0`
      (`self.K2_AttachToComponent` (`/Game/MyContent/Blueprints/Character/BP_BaseCharacter.FirstPersonMesh` (`self.GetOwnerBaseCharacterRef`)) "GripPoint" "SnapToTarget" "SnapToTarget" "SnapToTarget")
      (`/Engine/EditorBlueprintResources/StandardMacros.IsValid` _returnvalue
        (:`Is Valid`
          (`EnhancedInputSubsystemInterface.AddMappingContext` _returnvalue "/Game/MyContent/Input/IMC_Weapons.IMC_Weapons" 1 (struct))
          (bind _asfirst_person_anim_bp (cast `/Game/MyContent/Assets/FirstPersonArms/Animations/FirstPerson_AnimBP` (`self.GetAnimInstance` (`/Game/MyContent/Blueprints/Character/BP_BaseCharacter.FirstPersonMesh` (`self.GetOwnerBaseCharacterRef`)))))
          (set `/Game/MyContent/Assets/FirstPersonArms/Animations/FirstPerson_AnimBP.HasRifle` true _asfirst_person_anim_bp))))))

(event `ShootOrder`
  (`self.ShootValuesOnClient`))

(event `ShootValuesOnClient`
  (bind _returnvalue (`PlayerCameraManager.GetCameraRotation` (`PlayerController.PlayerCameraManager` (`/Game/MyContent/Blueprints/Character/BP_BaseCharacter.GetPlayerControllerRef` (`self.GetOwnerBaseCharacterRef`)))))
  (bind _returnvalue_2 (+ (`Actor.K2_GetActorLocation` (`self.GetOwner`)) (`KismetMathLibrary.GreaterGreater_VectorRotator` (`self.ProjectileOffset`) _returnvalue)))
  ;[0.01387 0 1] Comment
  (`self.ShootOnServer` _returnvalue_2 (+ _returnvalue_2 (* (`KismetMathLibrary.GetForwardVector` _returnvalue) (`self.FloatDistance`))) _returnvalue))

(event `ShootOnServer`
  (params (Start :type "Vector Structure") (End :type "Vector Structure") (Rotation :type "Rotator Structure"))
  (bind (_outhit _returnvalue) (`KismetSystemLibrary.SphereTraceSingle` :`Start` Start :`End` End :`Radius` (`self.FloatShootRadius`) :`TraceChannel` "TraceTypeQuery1" :`DrawDebugType` "ForDuration" :`DrawTime` 1.0))
  (`/Game/MyContent/Blueprints/Character/BP_BaseCharacter.OutOfAmmo` (`self.BaseCharacter`))
  (if _returnvalue
    (`self.ShootedMulticast` Start Rotation)
    (`KismetSystemLibrary.Delay` (`self.ImpactTime`))
    (if (`KismetSystemLibrary.DoesImplementInterface` (`.HitActor` (`GameplayStatics.BreakHitResult` _outhit)) "/Game/MyContent/Blueprints/BPI_HitInterface.BPI_HitInterface_C")
      ;[1 1 1] TODO NEW SYSTEM
      (message `/Game/MyContent/Blueprints/BPI_HitInterface.GetHitObject` (`.HitActor` (`GameplayStatics.BreakHitResult` _outhit)) (`self.NewCurrentTypeOfArrow`))
      (else
        (`self.SpawnStaticArrow` (`.ImpactPoint` (`GameplayStatics.BreakHitResult` _outhit)))))
    (else
      (`self.ShootedMulticast` Start Rotation))))

(event `ShootedMulticast`
  (params (SpawnPoint :type "Vector Structure") (Rotation :type "Rotator Structure"))
  ;[1 0 0.8976] TODO
  (`|SpawnActorFromClass` (`.VisualProjectile` (defaults `Object` (`self.NewCurrentTypeOfArrow`))) (`KismetMathLibrary.MakeTransform` SpawnPoint Rotation) "Undefined" "MultiplyWithRoot" null null))

(fn `ArrrowHits`
  (params (ActorHit :type "Actor Object Reference") (HitPoint :type "Vector Structure"))
  (locals (l_ActorHits :type "Actor Object Reference") (l_HitPoint :type "Vector Structure"))
  (set `local.l_ActorHits` ActorHit)
  (set `local.l_HitPoint` HitPoint)
  (switch `/Game/MyContent/Blueprints/E_Arrow` (`self.CurrentTypeOfArrow`)
    (:`NewEnumerator0`
      (`self.NormalArrowHit` (`local.l_ActorHits`) (`local.l_HitPoint`)))))

(fn `GetOwnerBaseCharacterRef`
  (returns (BaseCharacter :type "/Game/MyContent/Blueprints/Character/BP_BaseCharacter Object Reference"))
  (`self.BaseCharacter`
    (:`then`
      _)
    (:`else`
      (bind _asbp_base_character (cast `/Game/MyContent/Blueprints/Character/BP_BaseCharacter` (`self.GetOwner`)))
      (set `self.BaseCharacter` _asbp_base_character)))
  (return (`self.BaseCharacter`)))

(fn `NormalArrowHit`
  (params (ActorHit :type "Actor Object Reference") (HitPoint :type "Vector Structure"))
  (if (`KismetSystemLibrary.DoesImplementInterface` ActorHit "/Game/MyContent/Blueprints/BPI_HitInterface.BPI_HitInterface_C")
    (`|SpawnActorFromClass` "/Game/MyContent/Blueprints/Collectables/BP_ArrowCollectable.BP_ArrowCollectable_C" (`KismetMathLibrary.MakeTransform` HitPoint) "Undefined" "MultiplyWithRoot" null "NewEnumerator0" null)))

(fn `SpawnStaticArrow`
  (params (Location :type "Vector Structure"))
  (`|SpawnActorFromClass` (`.VisualCollectable` (defaults `Object` (`self.NewCurrentTypeOfArrow`))) (`KismetMathLibrary.MakeTransform` Location) "Undefined" "MultiplyWithRoot" null "NewEnumerator0" null))