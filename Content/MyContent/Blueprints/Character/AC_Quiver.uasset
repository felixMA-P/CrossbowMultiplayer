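; AC_Quiver is a quiver component that tracks a character's arrow ammo by arrow type.
; An Ammo map holds a count per type, with functions to read it, check that at least one arrow remains, and add arrows singly or in batches.
; RechargeArrow takes one arrow of the requested type and reports whether one was available.
; It runs no event logic, only these functions.
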(fn `AddArrows`
  (params (ArrowType :type "/Game/MyContent/Blueprints/E_Arrow Enum" :default "NewEnumerator0") (Number :type Integer))
  (`BlueprintMapLibrary.Map_Add` (`self.Ammo`) ArrowType (+ Number (`BlueprintMapLibrary.Map_Find` (`self.Ammo`) ArrowType))))

(fn `EnoughAmmoOfType`
  (params (Type :type "/Game/MyContent/Blueprints/E_Arrow Enum" :default "NewEnumerator0"))
  (returns (IsEnough :type Boolean))
  (bind _numberofarrows (`self.GetCurrentAmmoOfType` Type))
  (return (>= _numberofarrows 1)))

(fn `GetCurrentAmmoOfType`
  (params (Type :type "/Game/MyContent/Blueprints/E_Arrow Enum" :default "NewEnumerator0"))
  (returns (NumberOfArrows :type Integer))
  (return (`BlueprintMapLibrary.Map_Find` (`self.Ammo`) Type)))

(fn `RechargeArrow`
  (params (TypeOfArrow :type "/Game/MyContent/Blueprints/E_Arrow Enum" :default "NewEnumerator0"))
  (returns (Succes :type Boolean))
  (bind _value (`BlueprintMapLibrary.Map_Find` (`self.Ammo`) TypeOfArrow))
  (if (>= _value 1)
    (`BlueprintMapLibrary.Map_Add` (`self.Ammo`) TypeOfArrow (- _value 1))
    (return true)
    (else
      (return false))))

(fn `SaveArrow`
  (params (Type :type "/Game/MyContent/Blueprints/E_Arrow Enum" :default "NewEnumerator0"))
  (bind _ammo (`self.Ammo`))
  (`BlueprintMapLibrary.Map_Add` _ammo Type (+ (`BlueprintMapLibrary.Map_Find` _ammo Type) 1)))